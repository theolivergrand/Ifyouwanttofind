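; Torch Blueprint that serves as a switchable light with a particle effect.
; It overrides SwitchLight to call the parent version, then activate or deactivate its particle system to match the on/off state.
; On BeginPlay it switches itself on after a short delay.
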(event `self.ReceiveBeginPlay`
  (`KismetSystemLibrary.Delay` 3.0)
  (`self.SwitchLight` true))

(fn `SwitchLight`
  (params (`On/Off` :type Boolean))
  (bind _particlesystem (`self.ParticleSystem`))
  (`parent.SwitchLight` `On/Off`)
  (if `On/Off`
    (`ActorComponent.Activate` _particlesystem false)
    (else
      (`ActorComponent.Deactivate` _particlesystem))))

(fn `UserConstructionScript`
  (`parent.UserConstructionScript`))