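; Base lamp actor whose point light switches on and off, with optional proximity activation.
; SwitchLight stores the state and sets the light intensity to either MyIntensity or zero.
; When Autoswtich is set, Sphere overlaps turn the light on at entry and off at exit; it starts off on BeginPlay.
; A self-calling repeat event, commented as lamp blinking, calls SwitchLight after random delays, but nothing here starts it.
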(event `repeat`
  (params (`On/Off` :type Boolean))
  ;[1 1 1] Мигание лампы
  (`KismetSystemLibrary.Delay` (`KismetMathLibrary.RandomFloatInRange` 1.0 3.0))
  (`self.SwitchLight` (not (`self.On/Off`)))
  (`self.Repeat` false))

(event `self.ReceiveBeginPlay`
  (`self.SwitchLight` false))

(event `self.Sphere.OnComponentBeginOverlap`
  (params (OverlappedComponent :type "PrimitiveComponent Object Reference") (OtherActor :type "Actor Object Reference") (OtherComp :type "PrimitiveComponent Object Reference") (OtherBodyIndex :type Integer) (bFromSweep :type Boolean) (SweepResult :type "HitResult Structure (by ref)"))
  (if (`self.autoswtich`)
    (`self.SwitchLight` true)))

(event `self.Sphere.OnComponentEndOverlap`
  (params (OverlappedComponent :type "PrimitiveComponent Object Reference") (OtherActor :type "Actor Object Reference") (OtherComp :type "PrimitiveComponent Object Reference") (OtherBodyIndex :type Integer))
  (if (`self.autoswtich`)
    (`self.SwitchLight` false)))

(fn `SwitchLight`
  (params (`On/Off` :type Boolean))
  (set `self.On/Off` `On/Off`)
  (if (`self.On/Off`)
    (`LightComponent.SetIntensity` (`self.PointLight`) (`self.My Intensity`))
    (else
      (`LightComponent.SetIntensity` (`self.PointLight`) 0.0))))

(fn `UserConstructionScript`)