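; Lamp Blueprint that blinks its point light on and off at random intervals.
; BeginPlay switches the light off and enters an endless loop in which the repeat event waits one to three seconds, toggles the light, then calls itself.
; SwitchLight stores the on/off state and sets the PointLight intensity to either MyIntensity or zero.
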(event `repeat`
  (params (`On/Off` :type Boolean))
  (`KismetSystemLibrary.Delay` (`KismetMathLibrary.RandomFloatInRange` 1.0 3.0) :!label _label)
  (`self.SwitchLight` (not (`self.On/Off`)))
  (`self.Repeat` false))

(event `self.ReceiveBeginPlay`
  (`self.SwitchLight` false)
  (goto _label))

(fn `SwitchLight`
  (params (`On/Off` :type Boolean))
  (set `self.On/Off` `On/Off`)
  (if (`self.On/Off`)
    (`LightComponent.SetIntensity` (`self.PointLight`) (`self.My Intensity`))
    (else
      (`LightComponent.SetIntensity` (`self.PointLight`) 0.0))))

(fn `UserConstructionScript`)